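; BP_Skull_top is a modular human skeleton piece for the upper skull and its top teeth, each shown or hidden individually.
; The construction script sets visibility on the skull mesh and each tooth mesh from a matching boolean, without propagating to child components.
; The left-side top teeth read variables with a BOTTOM suffix, while the skull and other teeth use TOP.
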(fn ConstructionScript
  ;[1 1 1] SKULL TOP
  (Rendering|SetVisibility (Variables|Default|GetSM_Skull_top) (Variables|SKULL|GetSkull%20[TOP]) false)
  ;[1 1 1] TOOTHES TOP
  (Rendering|SetVisibility (Variables|Default|GetSM_Tooth_Top_1_1) (Variables|TOOTHES|GetTooth%201-1%20[TOP]) false)
  (Rendering|SetVisibility (Variables|Default|GetSM_Tooth_Top_2_r) (Variables|TOOTHES|GetTooth%202-R%20[TOP]) false)
  (Rendering|SetVisibility (Variables|Default|GetSM_Tooth_Top_3_r) (Variables|TOOTHES|GetTooth%203-R%20[TOP]) false)
  (Rendering|SetVisibility (Variables|Default|GetSM_Tooth_Top_4_r) (Variables|TOOTHES|GetTooth%204-R%20[TOP]) false)
  (Rendering|SetVisibility (Variables|Default|GetSM_Tooth_Top_5_r) (Variables|TOOTHES|GetTooth%205-R%20[TOP]) false)
  (Rendering|SetVisibility (Variables|Default|GetSM_Tooth_Top_6_r) (Variables|TOOTHES|GetTooth%206-R%20[TOP]) false)
  (Rendering|SetVisibility (Variables|Default|GetSM_Tooth_Top_7_r) (Variables|TOOTHES|GetTooth%207-R%20[TOP]) false)
  (Rendering|SetVisibility (Variables|Default|GetSM_Tooth_Top_8_r) (Variables|TOOTHES|GetTooth%208-R%20[TOP]) false)
  (Rendering|SetVisibility (Variables|Default|GetSM_Tooth_Top_2_L) (Variables|TOOTHES|GetTooth%202-L%20[BOTTOM]) false)
  (Rendering|SetVisibility (Variables|Default|GetSM_Tooth_Top_3_L) (Variables|TOOTHES|GetTooth%203-L%20[BOTTOM]) false)
  (Rendering|SetVisibility (Variables|Default|GetSM_Tooth_Top_4_L) (Variables|TOOTHES|GetTooth%204-L%20[BOTTOM]) false)
  (Rendering|SetVisibility (Variables|Default|GetSM_Tooth_Top_5_L) (Variables|TOOTHES|GetTooth%205-L%20[BOTTOM]) false)
  (Rendering|SetVisibility (Variables|Default|GetSM_Tooth_Top_6_L) (Variables|TOOTHES|GetTooth%206-L%20[BOTTOM]) false)
  (Rendering|SetVisibility (Variables|Default|GetSM_Tooth_Top_7_L) (Variables|TOOTHES|GetTooth%207-L%20[BOTTOM]) false)
  (Rendering|SetVisibility (Variables|Default|GetSM_Tooth_Top_8_L) (Variables|TOOTHES|GetTooth%208-L%20[BOTTOM]) false))