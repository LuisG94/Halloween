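; BP_Skull_full is a modular human skull Blueprint whose cranium, mandible and individual teeth can be shown or hidden.
; Its construction script runs three sub-graphs in turn, covering the skull parts, the top teeth and the bottom teeth.
; Each sub-graph sets component visibility from a matching variable without propagating to children, so hiding one part leaves its attached components unaffected.
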(fn ConstructionScript
  (|SKULL)
  (|ToothesTop)
  (|ToothesBottom))