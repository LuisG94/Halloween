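; Modular ceiling wire actor from the sewer system kit that builds a wire along an editable spline.
; The construction script adds a spline mesh between each pair of neighboring points, using their local locations and tangents to bend it along the curve.
; A second pass places a static mesh section at every point, with its rotation derived from the spline tangent.
; It has no runtime logic.
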(event EventBeginPlay)

(event Collision|EventActorBeginOverlap
  (params (OtherActor :type Actor%20Object%20Reference)))

(event EventTick
  (params (DeltaSeconds :type Float%20%28single-precision%29)))

(fn ConstructionScript
  (bind _spline (Variables|Default|GetSpline))
  (Utilities|FlowControl|Sequence
    (:then_0
      (for _index (range 0 (- (Spline|GetNumberOfSplinePoints (Variables|Default|GetSpline)) 2))
        ;[1 1 1] Add Wire Segment
        (bind _returnvalue (AddComponent|AddSplineMeshComponent false))
        ;[1 1 1] Align Wire to Spline
        (SplineMesh|SetStartandEnd _returnvalue (.Location (Spline|GetLocationandTangentatSplinePoint _spline _index "Local")) (.Tangent (Spline|GetLocationandTangentatSplinePoint _spline _index "Local")) (.Location (Spline|GetLocationandTangentatSplinePoint _spline (+ _index 1) "Local")) (.Tangent (Spline|GetLocationandTangentatSplinePoint _spline (+ _index 1) "Local")) true :!class /Script/Engine.SplineMeshComponent)))
    (:then_1
      (for _index_2 (range 0 (- (Spline|GetNumberOfSplinePoints (Variables|Default|GetSpline)) 1))
        ;[1 1 1] Add Wire Section
        (AddComponent|AddStaticMeshComponent false (Math|Transform|MakeTransform (.Location (Spline|GetLocationandTangentatSplinePoint (Variables|Default|GetSpline) _index_2 "Local")) (Math|Rotator|MakeRotationfromAxes (.Tangent (Spline|GetLocationandTangentatSplinePoint (Variables|Default|GetSpline) _index_2 "Local")) "0, 0, 0" "0, 0, 0") "1,1,1"))))))