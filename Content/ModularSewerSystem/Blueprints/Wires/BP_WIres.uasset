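; BP_WIres is a spline-based wire and cable placement actor from the modular sewer system, built entirely in the construction script.
; It adds a spline mesh for each segment between spline points, with WireType selecting one of seven wire meshes and its matching connector mesh.
; Optional connectors align to the spline ends: the start takes only the first point's rotation, the end takes the last point's transform, and disabled ones are destroyed.
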(event EventBeginPlay)

(event Collision|EventActorBeginOverlap
  (params (OtherActor :type Actor%20Object%20Reference)))

(event EventTick
  (params (DeltaSeconds :type Float%20%28single-precision%29)))

(fn ConstructionScript
  (bind _startconnector (Variables|Default|GetStartConnector))
  (bind _spline (Variables|Default|GetSpline))
  (bind _endconnector (Variables|Default|GetEndConnector))
  (for _index (range 0 (- (Spline|GetNumberOfSplinePoints (Variables|Default|GetSpline)) 2))
    (bind _returnvalue (AddComponent|AddSplineMeshComponent false))
    ;[1 1 1] Set Wire Type
    (switch int (Variables|Default|GetWireType)
      (:0
        (Components|StaticMesh|SetStaticMesh _returnvalue "/Game/ModularSewerSystem/Models/Detail/Wires/SM_YellowWire.SM_YellowWire")
        (Components|StaticMesh|SetStaticMesh _startconnector "/Game/ModularSewerSystem/Models/Detail/Wires/SM_YellowWire_connector.SM_YellowWire_connector")
        (Components|StaticMesh|SetStaticMesh _endconnector "/Game/ModularSewerSystem/Models/Detail/Wires/SM_YellowWire_connector.SM_YellowWire_connector"))
      (:1
        (Components|StaticMesh|SetStaticMesh _returnvalue "/Game/ModularSewerSystem/Models/Detail/Wires/SM_BlackWire.SM_BlackWire")
        (Components|StaticMesh|SetStaticMesh _startconnector "/Game/ModularSewerSystem/Models/Detail/Wires/SM_BlackWire_Connector.SM_BlackWire_Connector")
        (Components|StaticMesh|SetStaticMesh _endconnector "/Game/ModularSewerSystem/Models/Detail/Wires/SM_BlackWire_Connector.SM_BlackWire_Connector"))
      (:2
        (Components|StaticMesh|SetStaticMesh _returnvalue "/Game/ModularSewerSystem/Models/Detail/Wires/SM_PowerCable.SM_PowerCable")
        (Components|StaticMesh|SetStaticMesh _startconnector "/Game/ModularSewerSystem/Models/Detail/Wires/SM_PowerCable_Connector.SM_PowerCable_Connector")
        (Components|StaticMesh|SetStaticMesh _endconnector "/Game/ModularSewerSystem/Models/Detail/Wires/SM_PowerCable_Connector.SM_PowerCable_Connector"))
      (:3
        (Components|StaticMesh|SetStaticMesh _returnvalue "/Game/ModularSewerSystem/Models/Detail/Wires/SM_BigCable.SM_BigCable")
        (Components|StaticMesh|SetStaticMesh _startconnector "/Game/ModularSewerSystem/Models/Detail/Wires/SM_BigCable_Connector.SM_BigCable_Connector")
        (Components|StaticMesh|SetStaticMesh _endconnector "/Game/ModularSewerSystem/Models/Detail/Wires/SM_BigCable_Connector.SM_BigCable_Connector"))
      (:4
        (Components|StaticMesh|SetStaticMesh _returnvalue "/Game/ModularSewerSystem/Models/Detail/Wires/SM_HangingWireBundle.SM_HangingWireBundle")
        (Components|StaticMesh|SetStaticMesh _startconnector "/Game/ModularSewerSystem/Models/Detail/Wires/SM_HangingWireBundle_Connector.SM_HangingWireBundle_Connector")
        (Components|StaticMesh|SetStaticMesh _endconnector "/Game/ModularSewerSystem/Models/Detail/Wires/SM_HangingWireBundle_Connector.SM_HangingWireBundle_Connector"))
      (:5
        (Components|StaticMesh|SetStaticMesh _returnvalue "/Game/ModularSewerSystem/Models/Detail/Wires/SM_MetalWire.SM_MetalWire")
        (Components|StaticMesh|SetStaticMesh _startconnector "/Game/ModularSewerSystem/Models/Detail/Wires/SM_MetalWire_Connector.SM_MetalWire_Connector")
        (Components|StaticMesh|SetStaticMesh _endconnector "/Game/ModularSewerSystem/Models/Detail/Wires/SM_MetalWire_Connector.SM_MetalWire_Connector"))
      (:6
        (Components|StaticMesh|SetStaticMesh _returnvalue "/Game/ModularSewerSystem/Models/Detail/Wires/SM_WireBundle.SM_WireBundle")
        (Components|StaticMesh|SetStaticMesh _startconnector "/Game/ModularSewerSystem/Models/Detail/Wires/SM_WireBundle_Connector.SM_WireBundle_Connector")
        (Components|StaticMesh|SetStaticMesh _endconnector "/Game/ModularSewerSystem/Models/Detail/Wires/SM_WireBundle_Connector.SM_WireBundle_Connector")))
    ;[1 1 1] Align Wire To Spline
    (SplineMesh|SetStartandEnd _returnvalue (.Location (Spline|GetLocationandTangentatSplinePoint _spline _index "Local")) (.Tangent (Spline|GetLocationandTangentatSplinePoint _spline _index "Local")) (.Location (Spline|GetLocationandTangentatSplinePoint _spline (+ _index 1) "Local")) (.Tangent (Spline|GetLocationandTangentatSplinePoint _spline (+ _index 1) "Local")) true :!class /Script/Engine.SplineMeshComponent))
  ;[1 1 1] Start and End Connectors
  (if (Variables|Default|GetEnableEndCable)
    (Transformation|SetRelativeTransform (Variables|Default|GetEndConnector) (Spline|GetTransformatSplinePoint _spline (+ _index 1) "Local" false) false false)
    (else
      (Components|DestroyComponent (Variables|Default|GetEndConnector))))
  (if (Variables|Default|GetEnableStartCable)
    (Transformation|AddRelativeRotation (Variables|Default|GetStartConnector) (Spline|GetRotationatSplinePoint (Variables|Default|GetSpline) 0 "Local") false false)
    (else
      (Components|DestroyComponent (Variables|Default|GetStartConnector)))))