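; BP_SewerDoor is a configurable door prop for the modular sewer system, built entirely in its construction script with no runtime logic.
; Type variables select one of five door meshes and one of three frame meshes, and a flag toggles frame visibility.
; Alignment flags place DoorPivot on either side and flip HingePoint through offset and negative X scale.
; DoorRotation then sets the hinge yaw to pose the door.
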(event EventBeginPlay)

(event Collision|EventActorBeginOverlap
  (params (OtherActor :type Actor%20Object%20Reference)))

(event EventTick
  (params (DeltaSeconds :type Float%20%28single-precision%29)))

(fn ConstructionScript
  (bind _doorpivot (Variables|Default|GetDoorPivot))
  (bind _doorframe (Variables|Default|GetDoorFrame))
  (bind _hingepoint (Variables|Default|GetHingePoint))
  (bind _door (Variables|Default|GetDoor))
  (Utilities|FlowControl|Sequence
    (:then_0
      ;[1 1 1] Creates Door Mesh
      (switch int (Variables|Default|GetDoorType)
        (:Default
          (Components|StaticMesh|SetStaticMesh _door "/Game/ModularSewerSystem/Models/Detail/Doors/SM_Door_Blue.SM_Door_Blue" :!label _label))
        (:0
          (goto _label))
        (:1
          (Components|StaticMesh|SetStaticMesh _door "/Game/ModularSewerSystem/Models/Detail/Doors/SM_Door_Grate.SM_Door_Grate"))
        (:2
          (Components|StaticMesh|SetStaticMesh _door "/Game/ModularSewerSystem/Models/Detail/Doors/SM_Door_Metal.SM_Door_Metal"))
        (:3
          (Components|StaticMesh|SetStaticMesh _door "/Game/ModularSewerSystem/Models/Detail/Doors/SM_Door_White.SM_Door_White"))
        (:4
          (Components|StaticMesh|SetStaticMesh _door "/Game/ModularSewerSystem/Models/Detail/Doors/SM_Door_Window.SM_Door_Window"))))
    (:then_1
      ;[1 1 1] Creates Door Frame
      (switch int (Variables|Default|GetFrameType)
        (:Default
          (Components|StaticMesh|SetStaticMesh _doorframe "/Game/ModularSewerSystem/Models/Detail/Doors/SM_DoorFrame_A.SM_DoorFrame_A" :!label _label_2))
        (:0
          (goto _label_2))
        (:1
          (Components|StaticMesh|SetStaticMesh _doorframe "/Game/ModularSewerSystem/Models/Detail/Doors/SM_DoorFrame_B.SM_DoorFrame_B"))
        (:2
          (Components|StaticMesh|SetStaticMesh _doorframe "/Game/ModularSewerSystem/Models/Detail/Doors/SM_DoorFrame_C.SM_DoorFrame_C"))))
    (:then_2
      ;[1 1 1] Pivot
      (if (Variables|Default|GetDoorAlignment)
        (Transformation|SetRelativeLocationAndRotation _doorpivot "0,47.000000, 0" "0, 0, 0" false false)
        (else
          (Transformation|SetRelativeLocationAndRotation _doorpivot "0,-47.000000,0.000000" "0, 0, 0" false false))))
    (:then_3
      ;[1 1 1] Hinge
      (if (Variables|Default|GetHingeAlingment)
        (Transformation|SetRelativeTransform _hingepoint (Math|Transform|MakeTransform "-1.500000, 0, 0" "0, 0, 0" "-1.000000,1,1") false false)
        (else
          (Transformation|SetRelativeTransform _hingepoint (Math|Transform|MakeTransform "1.500000, 0, 0" "0, 0, 0" "1,1,1") false false))))
    (:then_4
      ;[1 1 1] Door Rotation
      (Transformation|SetRelativeRotation (Variables|Default|GetHingePoint) (Math|Rotator|MakeRotator 0.0 0.0 (Variables|Default|GetDoorRotation)) false false))
    (:then_5
      ;[1 1 1] Door Frame Visibility
      (Rendering|SetVisibility (Variables|Default|GetDoorFrame) (Variables|Default|GetDoorFrameEnabled) false))))