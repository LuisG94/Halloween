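; Spline-driven sewer pipe Blueprint that builds a run of pipe along its spline in the construction script.
; Each segment between spline points gets a spline mesh bent to the points' locations and tangents, using one of three straight pipe meshes chosen by PipeType.
; When PipeSectionEnable is set, a matching section mesh is placed at each interior point, rotated along the spline tangent.
; The event graph holds no runtime logic.
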(event EventBeginPlay)

(event Collision|EventActorBeginOverlap
  (params (OtherActor :type Actor%20Object%20Reference)))

(event EventTick
  (params (DeltaSeconds :type Float%20%28single-precision%29)))

(fn ConstructionScript
  (bind _spline (Variables|Default|GetSpline))
  (for _index (range 0 (- (Spline|GetNumberOfSplinePoints (Variables|Default|GetSpline)) 2))
    (Utilities|FlowControl|Sequence
      (:then_0
        ;[1 1 1] Pipe Placement
        (bind _returnvalue (AddComponent|AddSplineMeshComponent false))
        (switch int (Variables|Default|GetPipeType)
          (:0
            (Components|StaticMesh|SetStaticMesh _returnvalue "/Game/ModularSewerSystem/Models/Detail/Pipes/SM_PipeA_Straight.SM_PipeA_Straight"))
          (:1
            (Components|StaticMesh|SetStaticMesh _returnvalue "/Game/ModularSewerSystem/Models/Detail/Pipes/SM_PipeB_Straight.SM_PipeB_Straight"))
          (:2
            (Components|StaticMesh|SetStaticMesh _returnvalue "/Game/ModularSewerSystem/Models/Detail/Pipes/SM_PipeC_Straight.SM_PipeC_Straight")))
        ;[1 1 1] Alignment
        (SplineMesh|SetStartandEnd _returnvalue (.Location (Spline|GetLocationandTangentatSplinePoint _spline _index "Local")) (.Tangent (Spline|GetLocationandTangentatSplinePoint _spline _index "Local")) (.Location (Spline|GetLocationandTangentatSplinePoint _spline (+ _index 1) "Local")) (.Tangent (Spline|GetLocationandTangentatSplinePoint _spline (+ _index 1) "Local")) true :!class /Script/Engine.SplineMeshComponent))
      (:then_1
        ;[1 1 1] Pipe Section Switch
        (if (and (!= _index 0) (Variables|Default|GetPipeSectionEnable))
          ;[1 1 1] Pipe Section Placement
          (bind _returnvalue_2 (AddComponent|AddStaticMeshComponent false (Math|Transform|MakeTransform (.Location (Spline|GetLocationandTangentatSplinePoint _spline _index "Local")) (Math|Rotator|MakeRotationfromAxes (.Tangent (Spline|GetLocationandTangentatSplinePoint _spline _index "Local")) "0, 0, 0" "0, 0, 0") "1,1,1")))
          (switch int (Variables|Default|GetPipeType)
            (:0
              (Components|StaticMesh|SetStaticMesh _returnvalue_2 "/Game/ModularSewerSystem/Models/Detail/Pipes/SM_PipeA_Section.SM_PipeA_Section"))
            (:1
              (Components|StaticMesh|SetStaticMesh _returnvalue_2 "/Game/ModularSewerSystem/Models/Detail/Pipes/SM_PipeB_Section.SM_PipeB_Section"))
            (:2
              (Components|StaticMesh|SetStaticMesh _returnvalue_2 "/Game/ModularSewerSystem/Models/Detail/Pipes/SM_PipeC_Section.SM_PipeC_Section"))))))))