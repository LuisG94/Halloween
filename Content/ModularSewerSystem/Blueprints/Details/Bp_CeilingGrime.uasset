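; Construction-script Blueprint that scatters grime meshes and decals on surfaces above a resizable box, part of a modular sewer kit.
; For each grime count it traces upward from random points in the box against complex Visibility collision.
; Each hit gets a random mesh with random yaw and a normal-aligned decal, sharing a random scale.
; Each decal gets a dynamic material with a random scalar, though the parameter name is None.
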(event EventBeginPlay)

(event Collision|EventActorBeginOverlap
  (params (OtherActor :type Actor%20Object%20Reference)))

(event EventTick
  (params (DeltaSeconds :type Float%20%28single-precision%29)))

(fn ConstructionScript
  (bind _modellist (Variables|Default|GetModelList))
  (bind _box (Variables|Default|GetBox))
  (bind _returnvalue (Components|Box|GetUnscaledBoxExtent _box))
  (bind _returnvalue_2 (Transformation|GetWorldLocation _box))
  (bind _returnvalue_3 (Math|Random|RandomPointinBoundingBox _returnvalue_2 _returnvalue))
  (Components|Box|SetBoxExtent (Variables|Default|GetBox) (Math|Vector|MakeVector (Variables|Default|GetBoundExtent_X) (Variables|Default|GetBoundExtent_Y) 0.0) true)
  (for _index (range 0 (- (Variables|Default|GetGrimeAmount) 1))
    ;[1 1 1] Cast Up
    (bind (_outhit _returnvalue_4) (Collision|LineTraceByChannel _returnvalue_3 (+ _returnvalue_3 "0, 0,1000.000000") "TraceTypeQuery1" true 0 "ForOneFrame" true "(R=1.000000,G=0.000000,B=0.000000,A=1.000000)" "(R=0.000000,G=1.000000,B=0.000000,A=1.000000)" 1.0))
    (if _returnvalue_4
      (Utilities|FlowControl|Sequence
        (:then_0
          ;[1 1 1] Set Random Scale
          (Variables|Default|SetCurrentScale (Math|Random|RandomFloatinRange (Variables|Default|GetScaleMin) (Variables|Default|GetScaleMax))))
        (:then_1
          ;[1 1 1] Create Mesh
          (bind _returnvalue_5 (AddComponent|AddStaticMeshComponent false (Math|Transform|MakeTransform (- (.ImpactPoint (Collision|BreakHitResult _outhit)) (Transformation|GetActorLocation)) (Math|Rotator|MakeRotator 0.0 0.0 (Math|Random|RandomFloatinRange 0.0 3.6e+02)) (Math|Vector|MakeVector (Variables|Default|GetCurrentScale) (Variables|Default|GetCurrentScale) (Variables|Default|GetCurrentScale)))))
          (Components|StaticMesh|SetStaticMesh _returnvalue_5 (Utilities|Array|Get(acopy) _modellist (- (Math|Random|RandomIntegerinRange 1 (Utilities|Array|Length _modellist)) 1))))
        (:then_2
          ;[1 1 1] Create Decal
          (bind _returnvalue_6 (AddComponent|AddDecalComponent true (Math|Transform|MakeTransform (- (.ImpactPoint (Collision|BreakHitResult _outhit)) (Transformation|GetActorLocation)) (Math|Conversions|RotationFromXVector (* (.Normal (Collision|BreakHitResult _outhit)) -1.0)) (Math|Vector|MakeVector (Variables|Default|GetCurrentScale) (Variables|Default|GetCurrentScale) (Variables|Default|GetCurrentScale)))))
          (bind _returnvalue_7 (Rendering|Material|CreateDynamicMaterialInstance _returnvalue_6 :!class /Script/Engine.DecalComponent))
          (Rendering|Material|SetScalarParameterValue _returnvalue_7 "None" (Math|Conversions|ToFloat(Integer) (Math|Random|RandomIntegerinRange 0 3)) :!class /Script/Engine.MaterialInstanceDynamic))))))