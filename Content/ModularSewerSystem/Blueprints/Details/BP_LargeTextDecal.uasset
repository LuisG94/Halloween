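; BP_LargeTextDecal is a modular sewer detail actor that spells a text string as a row of projected letter decals.
; Its construction script splits up to 99 characters, matches each against an Alphabet array and adds one decal per match, offset by size and spacing.
; Each decal gets a small or large text material, with a dynamic instance selecting the glyph by Frame index and setting color, roughness, wear and chipping.
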(event EventBeginPlay)

(event Collision|EventActorBeginOverlap
  (params (OtherActor :type Actor%20Object%20Reference)))

(event EventTick
  (params (DeltaSeconds :type Float%20%28single-precision%29)))

(fn ConstructionScript
  (bind _textsize (Variables|Default|GetTextSize))
  (for (_array_element _array_index) (Utilities|String|GetCharacterArrayfromString (Utilities|String|GetSubstring (Variables|Default|GetText) 0 99))
    ;[1 1 1] Filter to A-Z 0-9
    (bind (_array_element_2 _array_index_2) (Utilities|Array|ForEachLoopwithBreak (Variables|Default|GetAlphabet))
      (:LoopBody
        (if (Utilities|Enum|Equal(Enum) _array_element_2 _array_element)
          ;[1 1 1] Create Decal
          (bind _returnvalue (AddComponent|AddDecalComponent false (Math|Transform|MakeTransform (Math|Vector|MakeVector 0.0 (* (Math|Conversions|ToFloat(Integer) _array_index) _textsize (Variables|Default|GetTextSpacing)) 0.0) "0.000000,0.000000,90.000000" (Math|Vector|MakeVector 1.0 _textsize _textsize))))
          ;[1 1 1] Set Material Type
          (switch int (Variables|Default|GetTextMaterial)
            (:Default
              (Rendering|Components|Decal|SetDecalMaterial _returnvalue "/Game/ModularSewerSystem/Materials/Decals/MI_LargeText.MI_LargeText" :!label _label))
            (:0
              (Rendering|Components|Decal|SetDecalMaterial _returnvalue "/Game/ModularSewerSystem/Materials/Decals/MI_SmallText.MI_SmallText"))
            (:1
              (goto _label)))
          (bind _returnvalue_2 (Rendering|Material|CreateDynamicMaterialInstance _returnvalue :!class /Script/Engine.DecalComponent))
          ;[1 1 1] Set Letter
          (Rendering|Material|SetScalarParameterValue _returnvalue_2 "Frame" (Math|Conversions|ToFloat(Integer) _array_index_2) :!class /Script/Engine.MaterialInstanceDynamic)
          ;[1 1 1] Set Color
          (Rendering|Material|SetVectorParameterValue _returnvalue_2 "Color" (Variables|Default|GetColor) :!class /Script/Engine.MaterialInstanceDynamic)
          ;[1 1 1] Set Roughness
          (Rendering|Material|SetScalarParameterValue _returnvalue_2 "Roughness" (Variables|Default|GetRoughness) :!class /Script/Engine.MaterialInstanceDynamic)
          ;[1 1 1] Set Wear
          (Rendering|Material|SetScalarParameterValue _returnvalue_2 "Wear" (Variables|Default|GetWear) :!class /Script/Engine.MaterialInstanceDynamic)
          ;[1 1 1] Set Chipping
          (Rendering|Material|SetScalarParameterValue _returnvalue_2 "Chipping" (Variables|Default|GetChipping) :!class /Script/Engine.MaterialInstanceDynamic))))))