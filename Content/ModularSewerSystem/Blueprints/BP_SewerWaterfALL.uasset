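; Sewer waterfall actor that builds a water mesh along an editable spline in its Construction Script, with no active runtime logic.
; It divides the spline into roughly 100-unit segments, adding a spline mesh for all but the last.
; WaterfallType picks one of four segment meshes.
; Each piece follows the spline's points and tangents, tapers in X scale from MinScale to MaxScale, and receives the chosen Material.
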(event EventBeginPlay)

(event Collision|EventActorBeginOverlap
  (params (OtherActor :type Actor%20Object%20Reference)))

(event EventTick
  (params (DeltaSeconds :type Float%20%28single-precision%29)))

(fn ConstructionScript
  (bind _material (Variables|Default|GetMaterial))
  (bind _spline (Variables|Default|GetSpline))
  (bind _minscale (Variables|Default|GetMinScale))
  (bind _maxscale (Variables|Default|GetMaxScale))
  (bind _spline_2 (Variables|Default|GetSpline))
  (bind _returnvalue (Spline|GetSplineLength _spline_2))
  (bind _returnvalue_2 (Spline|GetSplineLength _spline))
  (bind _returnvalue_3 (/ _returnvalue 1e+02))
  (bind _returnvalue_4 (Math|Float|Round _returnvalue_3))
  (bind _returnvalue_5 (Math|Conversions|ToFloat(Integer) _returnvalue_4))
  (bind _returnvalue_6 (/ _returnvalue _returnvalue_5))
  (for _index (range 0 (- _returnvalue_4 2))
    ;[1 1 1] Add Meshes
    (bind _returnvalue_7 (AddComponent|AddSplineMeshComponent false))
    (switch int (Variables|Default|GetWaterfallType)
      (:0
        (Components|StaticMesh|SetStaticMesh _returnvalue_7 "/Game/ModularSewerSystem/Models/Detail/Water/SM_WaterFall_A_Segment.SM_WaterFall_A_Segment"))
      (:1
        (Components|StaticMesh|SetStaticMesh _returnvalue_7 "/Game/ModularSewerSystem/Models/Detail/Water/SM_WaterFall_B_Segment.SM_WaterFall_B_Segment"))
      (:2
        (Components|StaticMesh|SetStaticMesh _returnvalue_7 "/Game/ModularSewerSystem/Models/Detail/Water/SM_WaterFall_C_Segment.SM_WaterFall_C_Segment"))
      (:3
        (Components|StaticMesh|SetStaticMesh _returnvalue_7 "/Game/ModularSewerSystem/Models/Detail/Water/SM_WaterFall_D_Segment.SM_WaterFall_D_Segment")))
    ;[1 1 1] Align to Spline
    (SplineMesh|SetStartandEnd _returnvalue_7 (Spline|GetLocationatDistanceAlongSpline _spline_2 (* _index _returnvalue_6) "Local") (Spline|GetTangentatDistanceAlongSpline _spline_2 (* _index _returnvalue_6) "Local") (Spline|GetLocationatDistanceAlongSpline _spline_2 (* (+ _index 1) _returnvalue_6) "Local") (Spline|GetTangentatDistanceAlongSpline _spline_2 (* (+ _index 1) _returnvalue_6) "Local") true :!class /Script/Engine.SplineMeshComponent)
    (Utilities|FlowControl|Sequence
      (:then_0
        ;[1 1 1] Scale the Start and End of the Spline
        (SplineMesh|SetStartScale _returnvalue_7 (Math|Vector2D|MakeVector2D (Math|Float|MapRangeClamped (/ (* _index _returnvalue_6) _returnvalue_2) 0.0 1.0 _minscale _maxscale) 1.0) true :!class /Script/Engine.SplineMeshComponent))
      (:then_1
        (SplineMesh|SetEndScale _returnvalue_7 (Math|Vector2D|MakeVector2D (Math|Float|MapRangeClamped (/ (* (+ _index 1) _returnvalue_6) _returnvalue_2) 0.0 1.0 _minscale _maxscale) 1.0) true :!class /Script/Engine.SplineMeshComponent))
      (:then_2
        ;[1 1 1] Set Material
        (Rendering|Material|SetMaterial _returnvalue_7 0 _material))
      (:then_3
        (Rendering|Material|SetMaterial _returnvalue_7 0 _material)))))