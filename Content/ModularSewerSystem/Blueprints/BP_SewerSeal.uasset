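; BP_SewerSeal is a modular sewer seal prop made of a frame and a hinged door, configured in the editor.
; The construction script uses DoorType to pick round or square frame and door meshes, defaulting to round.
; It then sets the Pivot's pitch from DoorRotation to pose the door open or closed.
; The event graph holds no active logic, so there is no runtime behavior.
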(event EventBeginPlay)

(event Collision|EventActorBeginOverlap
  (params (OtherActor :type Actor%20Object%20Reference)))

(event EventTick
  (params (DeltaSeconds :type Float%20%28single-precision%29)))

(fn ConstructionScript
  (bind _frame (Variables|Default|GetFrame))
  (bind _door (Variables|Default|GetDoor))
  (Utilities|FlowControl|Sequence
    (:then_0
      ;[1 1 1] Seal frame
      (switch int (Variables|Default|GetDoorType)
        (:Default
          (Components|StaticMesh|SetStaticMesh _frame "/Game/ModularSewerSystem/Models/Detail/Doors/SM_RoundSeal.SM_RoundSeal" :!label _label)
          ;[1 1 1] Seal Door
          (Components|StaticMesh|SetStaticMesh _door "/Game/ModularSewerSystem/Models/Detail/Doors/SM_RoundSeal_Door.SM_RoundSeal_Door"))
        (:0
          (goto _label))
        (:1
          (Components|StaticMesh|SetStaticMesh _frame "/Game/ModularSewerSystem/Models/Detail/Doors/SM_SquareSeal.SM_SquareSeal")
          (Components|StaticMesh|SetStaticMesh _door "/Game/ModularSewerSystem/Models/Detail/Doors/SM_SquareSeal_Door.SM_SquareSeal_Door"))))
    (:then_1
      ;[1 1 1] Door Rotation
      (Transformation|SetRelativeRotation (Variables|Default|GetPivot) (Math|Rotator|MakeRotator 0.0 (Variables|Default|GetDoorRotation) 0.0) false false))))