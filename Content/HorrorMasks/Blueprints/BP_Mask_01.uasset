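; BP_Mask_01 is a horror mask pickup that the ThirdPersonCharacter wears on overlap.
; It records its starting transform at BeginPlay, then on overlap attaches to the character mesh's Mask1 socket and disables its collision.
; Any mask already worn is first detached, teleported back to its stored start transform and given collision again, with the character's Mask variable tracking the current one.
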(event EventBeginPlay
  ;[1 1 1] Begin Play
  (Variables|Default|SetStartTransform (Transformation|GetActorTransform)))

(event Collision|EventActorBeginOverlap
  (params (OtherActor :type Actor%20Object%20Reference))
  ;[1 1 1] Begin Overlap
  (bind _asthird_person_character (Utilities|Casting|CastToThirdPersonCharacter OtherActor))
  (Utilities|IsValid (Variables|/Game/HorrorMasks/DemoAssets/ThirdPersonBP/Blueprints/ThirdPersonCharacter.ThirdPersonCharacter_C|GetMask _asthird_person_character)
    (:Is%20Valid
      (Transformation|DetachFromActor (Variables|/Game/HorrorMasks/DemoAssets/ThirdPersonBP/Blueprints/ThirdPersonCharacter.ThirdPersonCharacter_C|GetMask _asthird_person_character) "KeepWorld" "KeepWorld" "KeepWorld")
      (Transformation|SetActorTransform (Variables|/Game/HorrorMasks/DemoAssets/ThirdPersonBP/Blueprints/ThirdPersonCharacter.ThirdPersonCharacter_C|GetMask _asthird_person_character) (Variables|BP_Mask_01_C|GetStartTransform (Variables|/Game/HorrorMasks/DemoAssets/ThirdPersonBP/Blueprints/ThirdPersonCharacter.ThirdPersonCharacter_C|GetMask _asthird_person_character)) false true)
      (Collision|SetActorEnableCollision (Variables|/Game/HorrorMasks/DemoAssets/ThirdPersonBP/Blueprints/ThirdPersonCharacter.ThirdPersonCharacter_C|GetMask _asthird_person_character) true))
    (:Is%20Not%20Valid
      _))
  (Transformation|AttachComponentToComponent (Variables|/Script/Engine.Character|GetMesh _asthird_person_character) "Mask1" "SnapToTarget" "SnapToTarget" "SnapToTarget" true)
  (Collision|SetActorEnableCollision self false)
  (Variables|/Game/HorrorMasks/DemoAssets/ThirdPersonBP/Blueprints/ThirdPersonCharacter.ThirdPersonCharacter_C|SetMask _asthird_person_character self))

(fn ConstructionScript)